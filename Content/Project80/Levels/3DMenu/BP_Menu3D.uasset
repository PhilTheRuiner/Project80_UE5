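; BP_Menu3D is an in-world menu screen that links to other menu actors for camera-based navigation in a 3D menu.
; On BeginPlay it binds to its Menu3D widget's transition event and disables actor tick.
; A transition index picks an entry from LinkedMenus, then swaps collision from this menu to the target and smoothly blends the player's view to it.
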(event `self.ReceiveBeginPlay`
  (bind _asmenu_3d (cast `/Game/Project80/Levels/3DMenu/Widget/Menu3D` (`WidgetComponent.GetUserWidgetObject` (`self.Widget`))))
  (add `/Game/Project80/Levels/3DMenu/Widget/Menu3D.TransistionToLinkedMenu` _asmenu_3d (delegate `OnTransistion`))
  (`self.SetActorTickEnabled` false))

(event `OnTransistion`
  (params (MenuIndex :type Integer))
  (if (`KismetArrayLibrary.Array_IsValidIndex` (`self.LinkedMenus`) MenuIndex)
    (`self.TransistionTo` (`|GetArrayItem` (`self.LinkedMenus`) MenuIndex))))

(event `TransistionTo`
  (params (NewMenu :type "/Game/Project80/Levels/3DMenu/BP_Menu3D Object Reference"))
  (`self.SetActorEnableCollision` false)
  (`self.SetActorEnableCollision` NewMenu true)
  (`PlayerController.SetViewTargetWithBlend` (`GameplayStatics.GetPlayerController` 0) NewMenu 2.0 "VTBlend_EaseInOut" 2.0 false))

(fn `UserConstructionScript`)