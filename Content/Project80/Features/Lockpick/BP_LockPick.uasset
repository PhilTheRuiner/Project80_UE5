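; Lockpick minigame actor: the player angles a bobby pin and turns the lock until it opens, firing OnPicked and stopping tick.
; Construction picks a random unlock window sized by Difficulty and limits the scene capture to this actor.
; Each tick, pin closeness to that window caps lock rotation; hitting the cap shakes the pin via timeline.
; The pin moves only while lock input is idle, and the lock springs back when released.
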(event `InputAxis|RotateLock`
  (params (AxisValue :type "Float (single-precision)"))
  (bind _output_get (set `self.RotateLockAxis` AxisValue))
  (if (== _output_get 0.0)
    (`self.EndPinShake`)))

(event `InputAxis|RotatePin`
  (params (AxisValue :type "Float (single-precision)"))
  (`self.AllowPinRotation`
    (:`true`
      (`self.RotatePin` (* AxisValue -1.0)))))

(event `self.ReceiveTick`
  (params (DeltaSeconds :type "Float (single-precision)"))
  (`self.HandleTick` DeltaSeconds))

(event `BeginPinShake`
  (if (not (`self.PinShaking?`))
    (set `self.PinShaking?` true)
    (bind (_direction _pinoffset) (`Timeline|PinShakeTimeline` :!via `PlayFromStart` :!label _label)
      (:`Update`
        (`self.SetPinOffset` _pinoffset)))))

(event `EndPinShake`
  (if (`self.PinShaking?`)
    (set `self.PinShaking?` false)
    (`|ExecutionSequence`
      (:`then_0`
        (goto _label :!via `Stop`))
      (:`then_1`
        (`self.SetPinOffset` 0.0)))))

(fn `GetLockRotation`
  (returns (Rotation :type "Float (double-precision)"))
  (bind _relativerotation_roll (`KismetMathLibrary.BreakRotator` (`SceneComponent.RelativeRotation` (`self.InnerLock`))))
  (return _relativerotation_roll))

(fn `GetPinRotation`
  (returns (`Rotation X` :type "Float (double-precision)"))
  (bind _relativerotation_roll (`KismetMathLibrary.BreakRotator` (`SceneComponent.RelativeRotation` (`self.Bobbypin`))))
  (return _relativerotation_roll))

(fn `HandleTick`
  (params (DeltaSeconds :type "Float (double-precision)"))
  (`self.UpdateAllowedLockRotation`)
  (if (> (`self.RotateLockAxis`) 0.0)
    (`self.RotateLock` (* (`self.RotateLockAxis`) (`self.LockRotationSpeed`) (`local.DeltaSeconds`)))
    (elif (> (`self.GetLockRotation`) 0.0)
      (`self.RotateLock` (* -1.0 (`self.LockRotationSpeed`) (`local.DeltaSeconds`)))
      (if (< (`self.GetLockRotation`) 0.0)
        (`self.SetLockRotation` 0.0)))))

(fn `IsPinInUnlockRange?`
  (returns (ReturnValue :type Boolean))
  (return (`KismetMathLibrary.InRange_FloatFloat` (`self.GetPinRotation`) (`self.MinUnlockAngle`) (`self.MaxUnlockAngle`))))

(fn `RotateLock`
  (params (Rotation :type "Float (double-precision)"))
  (`|ExecutionSequence`
    (:`then_0`
      (if (> (`local.Rotation`) 0.0)
        (if (>= (+ (`local.Rotation`) (`self.GetLockRotation`)) (`self.MaxLockAngle`))
          (`self.SetLockRotation` (`self.MaxLockAngle`))
          (`self.OnPicked`)
          (`self.SetActorTickEnabled` false)
          (return)
          (elif (>= (+ (`local.Rotation`) (`self.GetLockRotation`)) (`self.AllowedLockRotation`))
            (`self.SetLockRotation` (`self.AllowedLockRotation`))
            (`self.BeginPinShake`)
            (return)))))
    (:`then_1`
      (`SceneComponent.K2_AddLocalRotation` (`self.InnerLock`) (`KismetMathLibrary.MakeRotator` (`local.Rotation`)) false true))))

(fn `RotatePin`
  (params (Rotation :type "Float (double-precision)"))
  (`SceneComponent.K2_SetRelativeRotation` (`self.Bobbypin`) (`KismetMathLibrary.MakeRotator` (`KismetMathLibrary.FClamp` (+ Rotation (`self.GetPinRotation`)) (* (`self.MaxPinAngle (absolute)`) -1.0) (`self.MaxPinAngle (absolute)`))) false true))

(fn `SetLockRotation`
  (params (Rotation :type "Float (double-precision)"))
  (`SceneComponent.K2_SetRelativeRotation` (`self.InnerLock`) (`KismetMathLibrary.MakeRotator` Rotation) false false))

(fn `SetPinOffset`
  (params (Offset :type "Float (double-precision)"))
  (bind _bobbypin (`self.Bobbypin`))
  (bind (_relativelocation_x _relativelocation_y _relativelocation_z) (`KismetMathLibrary.BreakVector` (`SceneComponent.RelativeLocation` _bobbypin)))
  (`SceneComponent.K2_SetRelativeLocation` _bobbypin (`KismetMathLibrary.MakeVector` _relativelocation_x (* Offset (`self.PinShakeAmount`)) _relativelocation_z) false true))

(fn `UpdateAllowedLockRotation`
  (locals (PinCloseness :type "Float (double-precision)") (PinAngleFromValid :type "Float (double-precision)"))
  (bind _returnvalue (- (`self.MinUnlockAngle`) (`self.GetPinRotation`)))
  (`|ExecutionSequence`
    (:`then_0`
      (if (`self.IsPinInUnlockRange?`)
        (set `local.PinCloseness` 1.0)
        (else
          (bind _output_get (set `local.PinAngleFromValid` (select `bool` (> _returnvalue 0.0) :`false` (- (`self.GetPinRotation`) (`self.MaxUnlockAngle`)) :`true` _returnvalue)))
          (set `local.PinCloseness` (- 1.0 (`KismetMathLibrary.FClamp` (/ _output_get (`self.MaxLockMoveAngle`))))))))
    (:`then_1`
      (set `self.AllowedLockRotation` (* (`local.PinCloseness`) (`self.MaxLockAngle`))))))

(fn `UserConstructionScript`
  (locals (UnlockHalfRange :type "Float (double-precision)") (UnlockAngle :type "Float (double-precision)"))
  (bind _returnvalue (- (`self.MaxPinAngle (absolute)`) (`local.UnlockHalfRange`)))
  (`SceneCaptureComponent.ShowOnlyActorComponents` (`self.SceneCaptureComponent2D`) self false)
  (set `local.UnlockHalfRange` (/ (select `/Game/Project80/Features/Lockpick/LockpickDifficulty` (`self.Difficulty`) :`NewEnumerator0` 15.0 :`NewEnumerator1` 10.0 :`NewEnumerator2` 5.0) 2.0))
  (set `local.UnlockAngle` (`KismetMathLibrary.RandomFloatInRange` (* _returnvalue -1.0) _returnvalue))
  (set `self.MinUnlockAngle` (- (`local.UnlockAngle`) (`local.UnlockHalfRange`)))
  (set `self.MaxUnlockAngle` (+ (`local.UnlockAngle`) (`local.UnlockHalfRange`)))
  (`SceneComponent.K2_SetRelativeRotation` (`self.BobbypinMin`) (`KismetMathLibrary.MakeRotator` (`self.MinUnlockAngle`)) false false)
  (`SceneComponent.K2_SetRelativeRotation` (`self.BobbypinMax`) (`KismetMathLibrary.MakeRotator` (`self.MaxUnlockAngle`)) false false))