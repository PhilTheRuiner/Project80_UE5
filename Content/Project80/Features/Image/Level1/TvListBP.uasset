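; TvListBP is an inspectable clue prop that shows a TvList widget when the player right-clicks near it.
; Entering its box saves the control rotation, enables input and opens a gate to a FlipFlop toggle.
; The toggle hides mesh and decal after a short delay and creates the widget with its clue, or reverses both.
; Leaving the box restores rotation and visibility, disables input and removes the widget.
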(event `self.ReceiveBeginPlay`)

(event `Key|RightMouseButton`
  (params (Key :type "Key Structure"))
  (:`Pressed`
    (`/Engine/EditorBlueprintResources/StandardMacros.Gate` true :!label _label
      (:`Exit`
        (`/Engine/EditorBlueprintResources/StandardMacros.FlipFlop`
          (:`A`
            (`KismetSystemLibrary.Delay` 0.2)
            (`SceneComponent.SetVisibility` (`self.StaticMesh`) false false)
            (`SceneComponent.SetVisibility` (`self.Decal`) false false)
            (`/Engine/EditorBlueprintResources/StandardMacros.IsValid` (`self.TvList`)
              (:`Is Not Valid`
                (bind _returnvalue (`|GenericCreateObject` "/Game/Project80/Features/Image/Level1/TvList.TvList_C" (`self.ShortName`)))
                (bind _output_get (set `self.TvList` _returnvalue))
                (`UserWidget.AddToViewport` _output_get 0))))
          (:`B`
            (`SceneComponent.SetVisibility` (`self.StaticMesh`) true false :!label _label_2)
            (`SceneComponent.SetVisibility` (`self.Decal`) true false)
            (`/Engine/EditorBlueprintResources/StandardMacros.IsValid` (`self.TvList`)
              (:`Is Valid`
                (`Widget.RemoveFromParent` (`self.TvList`))
                (set `self.TvList` null)))))))))

(event `self.Box.OnComponentBeginOverlap`
  (params (OverlappedComponent :type "PrimitiveComponent Object Reference") (OtherActor :type "Actor Object Reference") (OtherComp :type "PrimitiveComponent Object Reference") (OtherBodyIndex :type Integer) (bFromSweep :type Boolean) (SweepResult :type "HitResult Structure (by ref)"))
  (bind _astop_down_character (cast `/Game/Project80/Core/TopDownCharacter` (`GameplayStatics.GetPlayerCharacter` 0)))
  (bind _output_get (set `self.Player` _astop_down_character))
  (set `self.PlayerControlRotation` (`Pawn.GetControlRotation` _output_get))
  (`self.EnableInput` (`GameplayStatics.GetPlayerController` 0))
  (goto _label :!via `Open`))

(event `self.Box.OnComponentEndOverlap`
  (params (OverlappedComponent :type "PrimitiveComponent Object Reference") (OtherActor :type "Actor Object Reference") (OtherComp :type "PrimitiveComponent Object Reference") (OtherBodyIndex :type Integer))
  (`Controller.SetControlRotation` (`Pawn.GetController` (`self.Player`)) (`self.PlayerControlRotation`))
  (`self.DisableInput` (`GameplayStatics.GetPlayerController` 0))
  (goto _label_2))

(fn `UserConstructionScript`)