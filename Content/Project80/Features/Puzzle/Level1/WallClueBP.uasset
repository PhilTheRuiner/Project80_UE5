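; Wall clue actor for the Level 1 puzzle that opens a clue widget on right-click once its trigger box is overlapped.
; The overlap enables input and opens a gate; the click hides the mesh and decal, switches to UI input and creates the Picture widget.
; Exiting or completing collection restores visuals and game input and removes the widget.
; Only completion also destroys the box, preventing retriggering.
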(event `Key|RightMouseButton`
  (params (Key :type "Key Structure"))
  (:`Pressed`
    (`/Engine/EditorBlueprintResources/StandardMacros.Gate` true :!label _label
      (:`Exit`
        (`KismetSystemLibrary.Delay` 0.2)
        (`WidgetBlueprintLibrary.SetInputMode_UIOnlyEx` (`GameplayStatics.GetPlayerController` 0) (`self.Picture`))
        (`SceneComponent.SetVisibility` (`self.StaticMesh`) false false)
        (`SceneComponent.SetVisibility` (`self.Decal`) false false)
        (`/Engine/EditorBlueprintResources/StandardMacros.IsValid` (`self.Picture`)
          (:`Is Not Valid`
            (bind _returnvalue (`|GenericCreateObject` "/Game/Project80/Features/Puzzle/Level1/Picture.Picture_C" (`self.ShortName`)))
            (bind _output_get (set `self.Picture` _returnvalue))
            (`UserWidget.AddToViewport` _output_get 0)
            (add `Button.OnClicked` (`/Game/Project80/Features/Puzzle/Level1/Picture.Button_Exit` (`self.Picture`)) (delegate `OnClicked_ButtonExit`))
            (add `/Game/Project80/Features/Puzzle/Level1/Picture.EndCollected` (`self.Picture`) (delegate `End`))))))))

(event `self.Box.OnComponentBeginOverlap`
  (params (OverlappedComponent :type "PrimitiveComponent Object Reference") (OtherActor :type "Actor Object Reference") (OtherComp :type "PrimitiveComponent Object Reference") (OtherBodyIndex :type Integer) (bFromSweep :type Boolean) (SweepResult :type "HitResult Structure (by ref)"))
  (`self.EnableInput` (`GameplayStatics.GetPlayerController` 0))
  (goto _label :!via `Open`))

(event `End`
  (params (`IsEnd?` :type Boolean))
  (if `IsEnd?`
    (`WidgetBlueprintLibrary.SetInputMode_GameAndUIEx` (`GameplayStatics.GetPlayerController` 0) (`self.Picture`) "DoNotLock" false)
    (`self.DisableInput` (`GameplayStatics.GetPlayerController` 0))
    (`SceneComponent.SetVisibility` (`self.StaticMesh`) true false)
    (`SceneComponent.SetVisibility` (`self.Decal`) true false)
    (`/Engine/EditorBlueprintResources/StandardMacros.IsValid` (`self.Picture`)
      (:`Is Valid`
        (`Widget.RemoveFromParent` (`self.Picture`))
        (set `self.Picture` null)
        (`ActorComponent.K2_DestroyComponent` (`self.Box`))))))

(event `OnClicked_ButtonExit`
  (if true
    (`WidgetBlueprintLibrary.SetInputMode_GameAndUIEx` (`GameplayStatics.GetPlayerController` 0) (`self.Picture`) "DoNotLock" false)
    (`self.DisableInput` (`GameplayStatics.GetPlayerController` 0))
    (`SceneComponent.SetVisibility` (`self.StaticMesh`) true false)
    (`SceneComponent.SetVisibility` (`self.Decal`) true false)
    (`/Engine/EditorBlueprintResources/StandardMacros.IsValid` (`self.Picture`)
      (:`Is Valid`
        (`Widget.RemoveFromParent` (`self.Picture`))
        (set `self.Picture` null)))))

(fn `UserConstructionScript`)