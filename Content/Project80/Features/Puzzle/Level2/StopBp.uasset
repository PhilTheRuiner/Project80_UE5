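; StopBp is a level 2 puzzle trigger that halts the player with a StopW screen, then teleports them to a set point.
; Box overlap by any actor pauses the game, switches to UI-only input and creates the widget if none exists.
; The widget's End event moves the TopDownCharacter to the Arrow and removes the widget, without unpausing here.
; The construction script positions the Arrow from the TeleportLoaction transform.
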(event `self.Box.OnComponentBeginOverlap`
  (params (OverlappedComponent :type "PrimitiveComponent Object Reference") (OtherActor :type "Actor Object Reference") (OtherComp :type "PrimitiveComponent Object Reference") (OtherBodyIndex :type Integer) (bFromSweep :type Boolean) (SweepResult :type "HitResult Structure (by ref)"))
  (`GameplayStatics.SetGamePaused` true)
  (`WidgetBlueprintLibrary.SetInputMode_UIOnlyEx` (`GameplayStatics.GetPlayerController` 0) (`self.Lock`))
  (`/Engine/EditorBlueprintResources/StandardMacros.IsValid` (`self.Lock`)
    (:`Is Not Valid`
      (bind _returnvalue (`|GenericCreateObject` "/Game/Project80/Features/Puzzle/Level2/StopW.StopW_C"))
      (bind _output_get (set `self.Lock` _returnvalue))
      (`UserWidget.AddToViewport` _output_get 0)
      (add `/Game/Project80/Features/Puzzle/Level2/StopW.End` (`self.Lock`) (delegate `Teloport`)))))

(event `Teloport`
  (bind (_returnvalue_location _returnvalue_rotation) (`KismetMathLibrary.BreakTransform` (`SceneComponent.K2_GetComponentToWorld` (`self.Arrow`))))
  (bind _astop_down_character (cast `/Game/Project80/Core/TopDownCharacter` (`GameplayStatics.GetPlayerCharacter` 0)))
  (`SceneComponent.K2_SetWorldTransform` (`Actor.RootComponent` _astop_down_character) (`KismetMathLibrary.MakeTransform` _returnvalue_location _returnvalue_rotation) false true)
  (`Widget.RemoveFromParent` (`self.Lock`))
  (set `self.Lock` null))

(fn `UserConstructionScript`
  (`SceneComponent.K2_SetRelativeTransform` (`self.Arrow`) (`self.TeleportLoaction`) false false))