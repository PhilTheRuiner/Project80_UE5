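; Puzzle lock actor for Level 2 that opens a lock UI widget when the player right-clicks after entering its Box trigger.
; Box overlap enables input and opens a gate; the click then switches to UI-only input and creates the widget after a short delay.
; Both exit buttons restore Game-and-UI input, disable actor input and remove the widget.
; The second exit button, like EndCollected with IsEnd true, also destroys the trigger.
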(event `Key|RightMouseButton`
  (params (Key :type "Key Structure"))
  (:`Pressed`
    (`/Engine/EditorBlueprintResources/StandardMacros.Gate` true :!label _label
      (:`Exit`
        (`KismetSystemLibrary.Delay` 0.2)
        (`WidgetBlueprintLibrary.SetInputMode_UIOnlyEx` (`GameplayStatics.GetPlayerController` 0) (`self.Lock`))
        (`/Engine/EditorBlueprintResources/StandardMacros.IsValid` (`self.Lock`)
          (:`Is Not Valid`
            (bind _returnvalue (`|GenericCreateObject` "/Game/Project80/Features/Puzzle/Level2/LockWidget.LockWidget_C" (`self.ShortName`)))
            (bind _output_get (set `self.Lock` _returnvalue))
            (`UserWidget.AddToViewport` _output_get 0)
            (add `Button.OnClicked` (`/Game/Project80/Features/Puzzle/Level2/LockWidget.Button_Exit1` (`self.Lock`)) (delegate `OnClicked_ButtonExit1`))
            (add `Button.OnClicked` (`/Game/Project80/Features/Puzzle/Level2/LockWidget.Button_Exit2` (`self.Lock`)) (delegate `OnClicked_ButtonExit2`))))))))

(event `self.Box.OnComponentBeginOverlap`
  (params (OverlappedComponent :type "PrimitiveComponent Object Reference") (OtherActor :type "Actor Object Reference") (OtherComp :type "PrimitiveComponent Object Reference") (OtherBodyIndex :type Integer) (bFromSweep :type Boolean) (SweepResult :type "HitResult Structure (by ref)"))
  (`self.EnableInput` (`GameplayStatics.GetPlayerController` 0))
  (goto _label :!via `Open`))

(event `EndCollected`
  (params (`IsEnd?` :type Boolean))
  (if `IsEnd?`
    (`WidgetBlueprintLibrary.SetInputMode_GameAndUIEx` (`GameplayStatics.GetPlayerController` 0) (`self.Lock`) "DoNotLock" false)
    (`self.DisableInput` (`GameplayStatics.GetPlayerController` 0))
    (`/Engine/EditorBlueprintResources/StandardMacros.IsValid` (`self.Lock`)
      (:`Is Valid`
        (`Widget.RemoveFromParent` (`self.Lock`))
        (set `self.Lock` null)
        (`ActorComponent.K2_DestroyComponent` (`self.Box`))))))

(event `OnClicked_ButtonExit2`
  (if true
    (if true
      (`WidgetBlueprintLibrary.SetInputMode_GameAndUIEx` (`GameplayStatics.GetPlayerController` 0) (`self.Lock`) "DoNotLock" false)
      (`self.DisableInput` (`GameplayStatics.GetPlayerController` 0))
      (`/Engine/EditorBlueprintResources/StandardMacros.IsValid` (`self.Lock`)
        (:`Is Valid`
          (`Widget.RemoveFromParent` (`self.Lock`))
          (set `self.Lock` null)
          (`ActorComponent.K2_DestroyComponent` (`self.Box`)))))))

(event `OnClicked_ButtonExit1`
  (if true
    (`WidgetBlueprintLibrary.SetInputMode_GameAndUIEx` (`GameplayStatics.GetPlayerController` 0) (`self.Lock`) "DoNotLock" false)
    (`self.DisableInput` (`GameplayStatics.GetPlayerController` 0))
    (`/Engine/EditorBlueprintResources/StandardMacros.IsValid` (`self.Lock`)
      (:`Is Valid`
        (`Widget.RemoveFromParent` (`self.Lock`))
        (set `self.Lock` null)))))

(fn `UserConstructionScript`)